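; BP_WalkoutController is a controller Blueprint that routes player input to the walkout character.
; On BeginPlay it casts player character 0 to BP_WalkoutCharacter and caches the reference.
; Input events call that character to jump, move along its actor forward vector with a heavily scaled axis value, and apply yaw and pitch look input.
; It binds no strafe axis, and Tick is unused.
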(event EventBeginPlay
  (bind _asbp_walkout_character (Utilities|Casting|CastToBP_WalkoutCharacter (Game|GetPlayerCharacter 0)))
  (Variables|Default|SetWalkoutCharacter _asbp_walkout_character))

(event EventTick
  (params (DeltaSeconds :type Float%20%28single-precision%29)))

(event Input|ActionEvents|InputActionJump
  (params (Key :type Key%20Structure :default "None"))
  (:Pressed
    (Character|Jump (Variables|Default|GetWalkoutCharacter))))

(event Input|AxisEvents|InputAxisMove
  (params (AxisValue :type Float%20%28single-precision%29))
  (bind _walkoutcharacter (Variables|Default|GetWalkoutCharacter))
  (Pawn|Input|AddMovementInput _walkoutcharacter (Math|Vector|GetForwardVector (Transformation|GetActorRotation _walkoutcharacter)) (* AxisValue 1e+03) false))

(event Input|AxisEvents|InputAxisTurn
  (params (AxisValue :type Float%20%28single-precision%29))
  (Pawn|Input|AddControllerYawInput (Variables|Default|GetWalkoutCharacter) AxisValue))

(event Input|AxisEvents|InputAxisLookUp
  (params (AxisValue :type Float%20%28single-precision%29))
  (Pawn|Input|AddControllerPitchInput (Variables|Default|GetWalkoutCharacter) AxisValue))

(fn ConstructionScript)